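; INIC saddle module that passes every item-container structure in the world to UpdateINIC, whose logic lies outside this graph.
; Each Tick gathers the containers into SyncActors and, while the arrays differ, nests a loop that updates valid entries and removes invalid ones.
; When the arrays match, UpdateINIC reuses the inner loop's element, not the current one.
; On TestMapArea, BeginPlay enables debug prints and runs test console commands.
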(event `self.ReceiveBeginPlay`
  (`parent.ReceiveBeginPlay`)
  (bind _returnvalue (`VictoryCore.BPGetPrimaryMapName` null))
  (if (`KismetStringLibrary.EqualEqual_StrStr` _returnvalue "TestMapArea")
    (set `self.IsDebug` true)
    (`KismetSystemLibrary.Delay` null 1.0)
    (`KismetSystemLibrary.ExecuteConsoleCommand` null "gcm" null)
    (`KismetSystemLibrary.ExecuteConsoleCommand` null "giveitem /Game/PrimalEarth/CoreBlueprints/Items/Structures/Misc/PrimalItemStructure_Campfire.PrimalItemStructure_Campfire 1 0 0" null)
    (else
      (set `self.IsDebug` false))))

(event `self.ReceiveTick`
  (params (DeltaSeconds :type "Float (single-precision)"))
  (bind _isdebug (`self.IsDebug`))
  (bind _syncactors (`self.SyncActors`))
  (`parent.ReceiveTick` DeltaSeconds)
  (bind _outactors (`GameplayStatics.GetAllActorsOfClass` null "/Script/ShooterGame.PrimalStructureItemContainer"))
  (bind _output_get (set `self.WorldActors` _outactors))
  (bind _array_element (`/Game/Base/Macros/PrimalArkMacroLibrary.ForEachRefLoop` _output_get)
    (:`LoopBody`
      (`/Engine/EditorBlueprintResources/StandardMacros.IsValid` _array_element
        (:`Is Valid`
          (`KismetArrayLibrary.Array_AddUnique` _syncactors _array_element)
          (if (`KismetArrayLibrary.Array_Identical` _output_get _syncactors)
            (if _isdebug :!label _label
              (`KismetSystemLibrary.PrintString` null "In Sync" true true (struct :`G` 0.66 :`B` 1.0 :`A` 1.0) 0.5 "Sync In"))
            (bind _asprimal_structure_item_container (cast `PrimalStructureItemContainer` (stale _array_element_2)))
            (`/INIControl/Functions/NeverTouched/BPFL_INIC_Ammo .Update_INIC` (`PrimalAutocastFunctions.GameModeBaseToShooterGameMode` (`GameplayStatics.GetGameMode` null)) _asprimal_structure_item_container (`PrimalStructureItemContainer.MyInventoryComponent` _asprimal_structure_item_container) (`PrimalActor.bLoadedFromSaveGame` _asprimal_structure_item_container))
            (else
              (bind _array_element_2 (`/Game/Base/Macros/PrimalArkMacroLibrary.ForEachRefLoop` _syncactors)
                (:`LoopBody`
                  (`/Engine/EditorBlueprintResources/StandardMacros.IsValid` _array_element_2
                    (:`Is Valid`
                      (goto _label))
                    (:`Is Not Valid`
                      (`KismetArrayLibrary.Array_RemoveItem` _syncactors _array_element_2)
                      (if _isdebug
                        (`KismetSystemLibrary.PrintString` null "Out Of Sync" true true (struct :`G` 0.66 :`B` 1.0 :`A` 1.0) 0.5 "Sync Out")))))))))))))

(fn `UserConstructionScript`)